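; Player controller that flies the pawn as a free camera and triggers debug-style actions on the BP_MapGrid map.
; WASD presses and releases add to or subtract from a movement vector, which a looping timer-driven Move function applies each interval, scaled by delta time.
; A scroll axis drives height, clamped to a fixed range.
; R starts map navigation from the start room and F toggles map obfuscation.
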(event EventBeginPlay
  (Utilities|Time|SetTimerbyFunctionName self "Move" 0.016 true))

(event Input|KeyboardEvents|W
  (params (Key :type Key%20Structure))
  (bind _movespeed (Variables|Default|GetMoveSpeed))
  (:Pressed
    (Variables|Default|SetMovementVector (Math|Vector|MakeVector (+ _movespeed (.x (Variables|Default|GetMovementVector))) (.y (Variables|Default|GetMovementVector)) (.z (Variables|Default|GetMovementVector)))))
  (:Released
    (Variables|Default|SetMovementVector (Math|Vector|MakeVector (- (.x (Variables|Default|GetMovementVector)) _movespeed) (.y (Variables|Default|GetMovementVector)) (.z (Variables|Default|GetMovementVector))))))

(event Input|KeyboardEvents|S
  (params (Key :type Key%20Structure))
  (bind _movespeed (Variables|Default|GetMoveSpeed))
  (bind _returnvalue (* _movespeed -1.0))
  (:Pressed
    (Variables|Default|SetMovementVector (Math|Vector|MakeVector (+ (.x (Variables|Default|GetMovementVector)) _returnvalue) (.y (Variables|Default|GetMovementVector)) (.z (Variables|Default|GetMovementVector)))))
  (:Released
    (Variables|Default|SetMovementVector (Math|Vector|MakeVector (- (.x (Variables|Default|GetMovementVector)) _returnvalue) (.y (Variables|Default|GetMovementVector)) (.z (Variables|Default|GetMovementVector))))))

(event Input|KeyboardEvents|R
  (params (Key :type Key%20Structure))
  (:Pressed
    (bind _returnvalue (Actor|GetActorOfClass "/Game/Blueprints/BP_MapGrid.BP_MapGrid_C"))
    (Default|BeginNavigationfromStartRoom _returnvalue)))

(event Input|KeyboardEvents|A
  (params (Key :type Key%20Structure))
  (bind _movespeed (Variables|Default|GetMoveSpeed))
  (bind _returnvalue (* _movespeed -1.0))
  (:Pressed
    (Variables|Default|SetMovementVector (Math|Vector|MakeVector (.x (Variables|Default|GetMovementVector)) (+ (.y (Variables|Default|GetMovementVector)) _returnvalue) (.z (Variables|Default|GetMovementVector)))))
  (:Released
    (Variables|Default|SetMovementVector (Math|Vector|MakeVector (.x (Variables|Default|GetMovementVector)) (- (.y (Variables|Default|GetMovementVector)) _returnvalue) (.z (Variables|Default|GetMovementVector))))))

(event Input|KeyboardEvents|F
  (params (Key :type Key%20Structure))
  (:Pressed
    (bind _returnvalue (Actor|GetActorOfClass "/Game/Blueprints/BP_MapGrid.BP_MapGrid_C"))
    (Default|SetMapObfuscation _returnvalue (not (Variables|/Game/Blueprints/BP_MapGrid.BP_MapGrid_C|GetbIsMapObfuscated _returnvalue)))))

(event Input|KeyboardEvents|D
  (params (Key :type Key%20Structure))
  (bind _movespeed (Variables|Default|GetMoveSpeed))
  (:Pressed
    (Variables|Default|SetMovementVector (Math|Vector|MakeVector (.x (Variables|Default|GetMovementVector)) (+ (.y (Variables|Default|GetMovementVector)) _movespeed) (.z (Variables|Default|GetMovementVector)))))
  (:Released
    (Variables|Default|SetMovementVector (Math|Vector|MakeVector (.x (Variables|Default|GetMovementVector)) (- (.y (Variables|Default|GetMovementVector)) _movespeed) (.z (Variables|Default|GetMovementVector))))))

(fn ConstructionScript)

(fn Move
  (bind _returnvalue (Utilities|Time|GetWorldDeltaSeconds))
  (bind _returnvalue_2 (Game|Player|GetPlayerPawn 0))
  (bind _returnvalue_3 (Class|Actor|GetInputAxisKeyValue))
  (bind _movementvector (Variables|Default|GetMovementVector))
  (bind _scrollspeed (Variables|Default|GetScrollSpeed))
  (bind _returnvalue_4 (Transformation|GetActorLocation _returnvalue_2))
  (bind _returnvalue_5 (* _returnvalue_3 -1.0))
  (bind _returnvalue_6 (* _returnvalue_5 _scrollspeed))
  (bind _returnvalue_7 (Math|Vector|MakeVector (.x _movementvector) (.y _movementvector) _returnvalue_6))
  (bind _returnvalue_8 (* _returnvalue_7 _returnvalue))
  (bind _returnvalue_9 (+ _returnvalue_4 _returnvalue_8))
  (Transformation|SetActorLocation _returnvalue_2 (Math|Vector|MakeVector (.x _returnvalue_9) (.y _returnvalue_9) (Math|Float|Clamp(Float) (.z _returnvalue_9) 5e+02 1e+04)) false false))