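; Procedurally generates a branching room map, from a start room to a boss room, and begins navigation on BeginPlay.
; Spawns a jittered rows-by-lanes grid of BP_Room actors, with weighted-random types and levels scaling by row.
; Links each room straight ahead with chance-based diagonal branches, joining the first and last rows to the terminal rooms.
; Tracks the selected room and travelled path, starting obfuscated with the end room explored.
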(event EventBeginPlay
  (CallFunction|NormalizeRoomChances)
  (CallFunction|GenerateAllRooms)
  (CallFunction|CreateAllAttachements)
  (CallFunction|BeginNavigationfromStartRoom))

(fn ConstructionScript)

(fn GenerateAllRooms
  (bind _blockspacing (Variables|Generation|GetBlockSpacing))
  ;[0.2969 0.2969 0.2969] Outer Loop
  (for _index (range 0 (- (Variables|Generation|GetRows) 1))
    ;;[1 1 1] Inner Loop
    (for _index_2 (range 0 (- (Variables|Generation|GetLanes) 1))
      (bind _returnvalue (Game|SpawnActorfromClass "/Game/Blueprints/BP_Room.BP_Room_C" (Math|Conversions|ToTransform(Vector) (+ (Math|Vector|MakeVector (* _index _blockspacing) (* _index_2 _blockspacing) 0.0) (Transformation|GetActorLocation) (CallFunction|GetRandomVariance))) "AlwaysSpawn" 0 self 0)) ; Spawn a  block
      (Utilities|Array|AddUnique (Variables|Default|GetRoomArray) _returnvalue)
      (Default|SetRoomType _returnvalue (CallFunction|GetRandomWeightedRoomType))
      (EventDispatchers|BindEventtoSelected _returnvalue (EventDispatchers|CreateEvent :!event SelectRoom))
      (Default|Unexplore _returnvalue)
      (bind _returnvalue_2 (CallFunction|GetRoomLevel _index))
      (Default|SetLevel _returnvalue _returnvalue_2)))
  (CallFunction|PlaceTerminalRooms))

(fn GetRandomWeightedRoomType
  (bind _keys (Utilities|Map|Keys (Variables|Generation|GetRoomChances)))
  ;[1 1 1] Build the table of weighted odds
  (for _array_element _keys
    (if (> (.Value (Utilities|Map|Find (Variables|Generation|GetRoomChances) _array_element)) 0.0) ; If the value at key is > 0
      (bind _output_get (LocalVariables|SetRunningTotal (+ (LocalVariables|GetRunningTotal) (.Value (Utilities|Map|Find (Variables|Generation|GetRoomChances) _array_element)))))
      (Utilities|Map|Add (LocalVariables|GetOrderedMap) _array_element _output_get)))
  (LocalVariables|SetRandomVal (Math|Random|RandomFloatinRange 0.0 (LocalVariables|GetRunningTotal)))
  ;[1 1 1] Get the return room type based on a random value.
  (bind _keys_2 (Utilities|Map|Keys (LocalVariables|GetOrderedMap)))
  (for _array_element_2 _keys_2
    (if (< (- (LocalVariables|GetRandomVal) (.Value (Utilities|Map|Find (LocalVariables|GetOrderedMap) _array_element_2))) 0.0) ; If RV is less than the value at this Key
      (if (< (Math|Float|Absolute(Float) (- (LocalVariables|GetRandomVal) (.Value (Utilities|Map|Find (LocalVariables|GetOrderedMap) _array_element_2)))) (LocalVariables|GetDifference)) ; If the difference at RV is lesser than the difference at "Difference"
        (LocalVariables|SetDifference (Math|Float|Absolute(Float) (- (LocalVariables|GetRandomVal) (.Value (Utilities|Map|Find (LocalVariables|GetOrderedMap) _array_element_2)))))
        (LocalVariables|SetReturnRoomType _array_element_2))))
  (return (LocalVariables|GetReturnRoomType)))

(fn PlaceTerminalRooms
  (bind _lanes (Variables|Generation|GetLanes))
  (bind _roomarray (Variables|Default|GetRoomArray))
  (bind _returnvalue (/ _lanes 2))
  (if (== (Math|Integer|%(Integer) (Variables|Generation|GetLanes) 2) 1) ; If lanes are odd
    ;[1 1 1] Set Start Room Location if Lanes is odd.
    (LocalVariables|SetStartRoomLocation (Math|Vector|MakeVector (* (Variables|Generation|GetBlockSpacing) -1.5) (.y (Transformation|GetActorLocation (Utilities|Array|Get(acopy) (Variables|Default|GetRoomArray) (/ (Variables|Generation|GetLanes) 2)))) 0.0))
    (else
      ;[1 1 1] Set Start Room Location if Lanes is even.
      (LocalVariables|SetStartRoomLocation (Math|Vector|MakeVector (* (Variables|Generation|GetBlockSpacing) -1.5) (* (+ (.y (Transformation|GetActorLocation (Utilities|Array|Get(acopy) (Variables|Default|GetRoomArray) (- _returnvalue 1)))) (.y (Transformation|GetActorLocation (Utilities|Array|Get(acopy) (Variables|Default|GetRoomArray) _returnvalue)))) 0.5) 0.0))))
  ;[1 1 1] Set End Room Location
  (LocalVariables|SetEndRoomLocation (Math|Vector|MakeVector (+ (.x (Transformation|GetActorLocation (Utilities|Array|Get(acopy) _roomarray (Utilities|Array|LastIndex _roomarray)))) (Variables|Generation|GetBlockSpacing)) (.y (LocalVariables|GetStartRoomLocation)) (.z (LocalVariables|GetStartRoomLocation))))
  ;[1 1 1] Place Start room
  (bind _returnvalue_2 (Game|SpawnActorfromClass "/Game/Blueprints/BP_Room.BP_Room_C" (Math|Conversions|ToTransform(Vector) (LocalVariables|GetStartRoomLocation)) "AlwaysSpawn" 0 self 0)) ; Spawn a  block
  (bind _output_get (Variables|Default|SetStartRoom _returnvalue_2))
  (Default|SetRoomType _output_get "NewEnumerator1")
  (EventDispatchers|BindEventtoSelected _output_get (EventDispatchers|CreateEvent :!event SelectRoom))
  (Default|SetLevel _output_get)
  ;[1 1 1] Place Boss Room
  (bind _returnvalue_3 (Game|SpawnActorfromClass "/Game/Blueprints/BP_Room.BP_Room_C" (Math|Conversions|ToTransform(Vector) (LocalVariables|GetEndRoomLocation)) "AlwaysSpawn" 0 self 0)) ; Spawn a  block
  (bind _output_get_2 (Variables|Default|SetEndRoom _returnvalue_3))
  (Default|SetRoomType _output_get_2 "NewEnumerator2")
  (EventDispatchers|BindEventtoSelected _output_get_2 (EventDispatchers|CreateEvent :!event SelectRoom))
  (Default|Unexplore _output_get_2)
  (Default|SetLevel _output_get_2 (+ (Math|Float|Round (* (Variables|Generation|GetRows) (Variables|Generation|GetLevelScaling))) (Variables|Generation|GetLevel%20Variance))))

(fn GetRandomVariance
  (bind _positionvariance (Variables|Generation|GetPositionVariance))
  (return (Math|Vector|MakeVector (Math|Random|RandomFloatinRange (* (.x _positionvariance) -1.0) (.x _positionvariance)) (Math|Random|RandomFloatinRange (* (.y _positionvariance) -1.0) (.y _positionvariance)) 0.0)))

(fn CreateStartRoomAttachments
  (for _index (range 0 (- (Variables|Generation|GetLanes) 1))
    (Default|AddConnectedRoom (Variables|Default|GetStartRoom) (Utilities|Array|Get(acopy) (Variables|Default|GetRoomArray) _index))))

(fn CreateEndRoomAttachements
  (bind _roomarray (Variables|Default|GetRoomArray))
  (bind _returnvalue (Utilities|Array|Length _roomarray))
  (for _index (range (- _returnvalue (Variables|Generation|GetLanes)) (- _returnvalue 1))
    (Default|AddConnectedRoom (Utilities|Array|Get(acopy) (Variables|Default|GetRoomArray) _index) (Variables|Default|GetEndRoom))))

(fn CreateAllAttachements
  (bind _roomarray (Variables|Default|GetRoomArray))
  (for (_array_element _array_index) _roomarray
    ;[1 1 1] Default, linear connections.
    (if (Utilities|Array|IsValidIndex _roomarray (+ _array_index (Variables|Generation|GetLanes)))
      (Default|AddConnectedRoom _array_element (Utilities|Array|Get(acopy) _roomarray (+ _array_index (Variables|Generation|GetLanes))))
      ;[1 1 1] Extra connection generation
      (if (<= (Math|Random|RandomFloat) (Variables|Generation|GetMultiConnectionRoomChance))
        (if (== (Math|Integer|%(Integer) (+ _array_index 1) (Variables|Generation|GetLanes)) 0) ; If 0, then the room is on the right edge.
          (LocalVariables|SetExtraConnectionIndex (+ (- _array_index 1) (Variables|Generation|GetLanes)) :!label _label)
          (else
            (if (== (Math|Integer|%(Integer) (+ _array_index 1) (Variables|Generation|GetLanes)) 1) ; If 1 then the room is on the left edge.
              _
              (elif (<= (Math|Random|RandomFloat) (Variables|Generation|GetTripleConnectionChance)) ; If triple connection
                (Utilities|FlowControl|Sequence
                  (:then_0
                    (goto _label))
                  (:then_1
                    _))
                (elif (>= (Math|Random|RandomFloat) 0.5) ; Pick a side at random.
                  (goto _label)
                  (else
                    _))))
            (LocalVariables|SetExtraConnectionIndex (+ (+ _array_index 1) (Variables|Generation|GetLanes)))))
        (Default|AddConnectedRoom _array_element (Utilities|Array|Get(acopy) (Variables|Default|GetRoomArray) (LocalVariables|GetExtraConnectionIndex))))))
  (CallFunction|CreateStartRoomAttachments)
  (CallFunction|CreateEndRoomAttachements))

(fn SelectRoom
  (params (Room :type BP%20Room%20Object%20Reference))
  (Utilities|IsValid (Variables|Default|GetSelectedRoom)
    (:Is%20Valid
      (Default|Deselect (Variables|Default|GetSelectedRoom))
      (Default|SetTravelledPath (Variables|Default|GetSelectedRoom) Room))
    (:Is%20Not%20Valid
      _))
  (Variables|Default|SetSelectedRoom Room))

(fn NormalizeRoomChances
  (bind _keys (Utilities|Map|Keys (Variables|Generation|GetRoomChances)))
  ;[1 1 1] Get the highest value in the map
  (for _array_element _keys
    (if (> (.Value (Utilities|Map|Find (Variables|Generation|GetRoomChances) _array_element)) (LocalVariables|GetHighestVal))
      (LocalVariables|SetHighestVal (.Value (Utilities|Map|Find (Variables|Generation|GetRoomChances) _array_element)))))
  ;[1 1 1] Create a map normalized to the highest value.
  (for _array_element_2 _keys
    (Utilities|Map|Add (LocalVariables|GetNormalizedMap) _array_element_2 (/ (.Value (Utilities|Map|Find (Variables|Generation|GetRoomChances) _array_element_2)) (LocalVariables|GetHighestVal))))
  (Variables|Generation|SetRoomChances (LocalVariables|GetNormalizedMap)))

(fn BeginNavigationfromStartRoom
  (bind _startroom (Variables|Default|GetStartRoom))
  (for _array_element (Variables|Default|GetRoomArray)
    (Default|Reset _array_element))
  (Default|SetIsTravelOption _startroom true)
  (Default|Select _startroom)
  (Default|SetIsTravelOption _startroom false)
  (Default|Explore (Variables|Default|GetEndRoom))
  (CallFunction|SetMapObfuscation true))

(fn SetMapObfuscation
  (params (Obfuscation :type Boolean))
  (bind _output_get (Variables|Default|SetbIsMapObfuscated Obfuscation))
  (for _array_element (Variables|Default|GetRoomArray)
    (Default|SetObfuscation _array_element _output_get)))

(fn GetRoomLevel
  (params (CurrentRow :type Integer))
  (bind _output_get (LocalVariables|SetScaledBaseLevel (Math|Float|Round (* (+ CurrentRow 1) (Variables|Generation|GetLevelScaling)))))
  (return (+ _output_get (Math|Random|RandomIntegerinRange (select (< (- (LocalVariables|GetScaledBaseLevel) (Variables|Generation|GetLevel%20Variance)) 1) (* (- (LocalVariables|GetScaledBaseLevel) 1) -1) (* (Variables|Generation|GetLevel%20Variance) -1)) (Variables|Generation|GetLevel%20Variance)))))